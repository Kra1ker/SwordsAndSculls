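; BP_potion is a healing pickup that restores the player's health on overlap.
; On BeginPlay it caches the player BP_char and runs a Moving timeline that animates the Potion component's relative location.
; Overlapping Collision below max health adds HealingValue once, without clamping, and calls CallChangingHealth with the health ratio.
; A Taking timeline then moves the potion, with a delay in its update branch before the actor destroys itself.
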(event OnComponentBeginOverlap(Collision)
  (params (OverlappedComponent :type Primitive%20Component%20Object%20Reference) (OtherActor :type Actor%20Object%20Reference) (OtherComp :type Primitive%20Component%20Object%20Reference) (OtherBodyIndex :type Integer) (bFromSweep :type Boolean) (SweepResult :type Hit%20Result%20Structure%20%28by%20ref%29))
  (bind _bp_char (Variables|Default|GetBP%20char))
  (bind _bp_char_2 (Variables|Default|GetBP%20char))
  (bind _bp_char_3 (Variables|Default|GetBP%20char))
  (Utilities|Casting|CastToBP_char OtherActor)
  (if (not (>= (Variables|/Game/Blueprints/Character/BP_char.BP_char_C|GetHealth _bp_char_3) (Variables|/Game/Blueprints/Character/BP_char.BP_char_C|GetMax_Health _bp_char_3)))
    (Utilities|FlowControl|DoOnce false
      (:Completed
        (Variables|/Game/Blueprints/Character/BP_char.BP_char_C|SetHealth _bp_char (+ (Variables|/Game/Blueprints/Character/BP_char.BP_char_C|GetHealth _bp_char) (Variables|Default|GethealingValue)))
        (Default|CallChangingHealth _bp_char (/ (Variables|/Game/Blueprints/Character/BP_char.BP_char_C|GetHealth _bp_char_2) (Variables|/Game/Blueprints/Character/BP_char.BP_char_C|GetMax_Health _bp_char_2)))
        (bind _newtrack_0 (Timeline|Taking Play)
          (:Update
            (Transformation|SetRelativeLocation (Variables|Default|GetPotion) _newtrack_0 false false)
            (Utilities|FlowControl|Delay 0.4)
            (Actor|DestroyActor)))))))

(event EventBeginPlay
  (bind _asbp_char (Utilities|Casting|CastToBP_char (Game|GetPlayerCharacter 0)))
  (Variables|Default|SetBP%20char _asbp_char)
  (bind _newtrack_0 (Timeline|Moving Play)
    (:Update
      (Transformation|SetRelativeLocation (Variables|Default|GetPotion) _newtrack_0 false false))))

(event Collision|EventActorBeginOverlap
  (params (OtherActor :type Actor%20Object%20Reference)))

(event EventTick
  (params (DeltaSeconds :type Float%20%28single-precision%29)))

(fn ConstructionScript)