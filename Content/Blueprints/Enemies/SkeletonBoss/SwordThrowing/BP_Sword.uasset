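; Sword projectile for the skeleton boss's throw attack, meant to damage the player character and play a hit animation.
; Sphere overlap chains casts to BP_boss and BP_char, then requires the actor to differ from the just-stored boss, so as wired the hit branch cannot pass.
; That branch applies damage, stops the projectile, swaps the flying flipbook for a one-shot hit flipbook and destroys the sword after a short delay.
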(event OnComponentBeginOverlap(Sphere)
  (params (OverlappedComponent :type Primitive%20Component%20Object%20Reference) (OtherActor :type Actor%20Object%20Reference) (OtherComp :type Primitive%20Component%20Object%20Reference) (OtherBodyIndex :type Integer) (bFromSweep :type Boolean) (SweepResult :type Hit%20Result%20Structure%20%28by%20ref%29))
  (bind _projectilemovement (Variables|Default|GetProjectileMovement))
  (bind _fb_hit (Variables|Default|GetFB_Hit))
  (bind _asbp_boss (Utilities|Casting|CastToBP_boss OtherActor))
  (bind _output_get (Variables|Default|SetAs%20BP%20Boss _asbp_boss))
  (bind _asbp_char (Utilities|Casting|CastToBP_char OtherActor))
  (if (and (!= _output_get OtherActor) (!= self OtherActor))
    (Game|Damage|ApplyDamage _asbp_char 1e+01 0 0)
    (Rendering|SetVisibility (Variables|Default|GetFB_FlyingSword) false false)
    (Variables|/Script/Engine.ProjectileMovementComponent|SetProjectileGravityScale _projectilemovement 0.0)
    (Components|Movement|StopMovementImmediately _projectilemovement)
    (Rendering|SetVisibility _fb_hit true false)
    (Components|Timeline|SetPlayRate _fb_hit 1.0)
    (Components|Timeline|SetLooping _fb_hit false)
    (Utilities|FlowControl|Delay 0.35)
    (Actor|DestroyActor)))

(event EventBeginPlay)

(event Collision|EventActorBeginOverlap
  (params (OtherActor :type Actor%20Object%20Reference)))

(event EventTick
  (params (DeltaSeconds :type Float%20%28single-precision%29)))

(fn ConstructionScript)