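; BP_skelet is a 2D skeleton enemy that patrols back and forth, damages the player on contact, and can be killed.
; Despite its name, Follow runs each tick as a counter-based patrol, flipping the sprite at each limit.
; BoxHit overlaps apply damage, pass the skeleton's X to the player, and trigger a movement-locking attack.
; Incoming damage knocks it away from the player, then plays a hit reaction or death before destruction.
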(event OnComponentBeginOverlap(BoxHit)
  (params (OverlappedComponent :type Primitive%20Component%20Object%20Reference) (OtherActor :type Actor%20Object%20Reference) (OtherComp :type Primitive%20Component%20Object%20Reference) (OtherBodyIndex :type Integer) (bFromSweep :type Boolean) (SweepResult :type Hit%20Result%20Structure%20%28by%20ref%29))
  (bind _returnvalue (Components|GetOwner))
  (Utilities|IsValid _returnvalue
    (:Is%20Valid
      (if (not (== _returnvalue OtherActor))
        (bind _asbp_char (Utilities|Casting|CastToBP_char OtherActor))
        (Game|Damage|ApplyDamage _asbp_char 2e+01 0 0)
        (Variables|/Game/Blueprints/Character/BP_char.BP_char_C|SetEnemyPos (Variables|Default|GetChar) (.x (Transformation|GetWorldLocation (Variables|Default|GetSprite))))
        (if (and (and (not (Variables|Default|GetIsAttacking)) (AI|Components|NavMovement|IsMovingonGround (Variables|Character|GetCharacterMovement))) (Collision|IsOverlappingActor (Variables|Default|GetBoxHit) (Variables|Default|GetChar) :!class /Script/Engine.PrimitiveComponent))
          (Class|PaperZDAnimInstance|JumptoNode (Variables|/Script/PaperZD.PaperZDAnimationComponent|GetAnimInstance (Variables|Default|GetAnimationComponent)) "Attacking" "None")
          (Variables|Default|SetIsAttacking true)
          (Variables|Default|SetisMovementLock true)
          (Utilities|FlowControl|Delay 1.0)
          (Variables|Default|SetisMovementLock false)
          (Variables|Default|SetIsAttacking false))))))

(event Custom|Follow
  (if (not (Variables|Default|GetisMovementLock))
    (Math|Float|CompareFloat (Variables|Default|GetS1) (Variables|Default|GetS)
      (:>
        (Pawn|Input|AddMovementInput "-1.000000,0.000000,0.000000" 1.0 false)
        (Variables|Default|SetS1 (- (Variables|Default|GetS1) 1.0)))
      (:==
        (if (> (Variables|Default|GetS) 0.0)
          (Variables|Default|SetS (* (Variables|Default|GetS) -1.0))
          (Variables|Default|SetS1 0.0)
          (Transformation|SetRelativeRotation (Variables|Default|GetSprite) "0.000000,180.000000,0.000000" false false)
          (else
            (Variables|Default|SetS (* (Variables|Default|GetS) -1.0))
            (Variables|Default|SetS1 0.0)
            (Transformation|SetRelativeRotation (Variables|Default|GetSprite) "0, 0, 0" false false))))
      (:<
        (Pawn|Input|AddMovementInput "1.000000,0.000000,0.000000" 1.0 false)
        (Variables|Default|SetS1 (+ (Variables|Default|GetS1) 1.0))))))

(event EventBeginPlay
  (bind _asbp_char (Utilities|Casting|CastToBP_char (Game|GetPlayerCharacter 0)))
  (Variables|Default|SetChar _asbp_char))

(event Collision|EventActorBeginOverlap
  (params (OtherActor :type Actor%20Object%20Reference)))

(event EventTick
  (params (DeltaSeconds :type Float%20%28single-precision%29))
  (CallFunction|Follow))

(event Game|Damage|EventAnyDamage
  (params (Damage :type Float%20%28single-precision%29) (DamageType :type Damage%20Type%20Object%20Reference) (InstigatedBy :type Controller%20Object%20Reference) (DamageCauser :type Actor%20Object%20Reference))
  (if (not (Variables|Default|GetIsDeath))
    (Math|Float|CompareFloat (.x (Transformation|GetWorldLocation (Variables|/Script/Paper2D.PaperCharacter|GetSprite (Variables|Default|GetChar)))) (.x (Transformation|GetWorldLocation (Variables|Default|GetSprite)))
      (:>
        (Character|LaunchCharacter "-500.000000,0.000000,100.000000" true true))
      (:<
        (Character|LaunchCharacter "500.000000,0.000000,100.000000" true true)))
    (bind _output_get (Variables|Default|SetHealth (- (Variables|Default|GetHealth) Damage)))
    (Development|PrintString (Utilities|String|Append "Health skeleton:" (Utilities|String|ToString(Float) _output_get)))
    (if (>= (Variables|Default|GetHealth) 0.0)
      (Class|PaperZDAnimInstance|JumptoNode (Variables|/Script/PaperZD.PaperZDAnimationComponent|GetAnimInstance (Variables|Default|GetAnimationComponent)) "Hitting" "None")
      (Variables|Default|SetisMovementLock true)
      (Utilities|FlowControl|Delay 0.5)
      (Variables|Default|SetisMovementLock false)
      (else
        (Class|PaperZDAnimInstance|JumptoNode (Variables|/Script/PaperZD.PaperZDAnimationComponent|GetAnimInstance (Variables|Default|GetAnimationComponent)) "Death" "None")
        (Variables|Default|SetIsAttacking true)
        (Variables|Default|SetIsDeath true)
        (Variables|Default|SetisMovementLock true)
        (Utilities|FlowControl|Delay 1.0)
        (Actor|DestroyActor)))))

(fn ConstructionScript)