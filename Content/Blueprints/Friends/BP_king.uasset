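; BP_king is a king actor in the Friends folder that shows an interaction widget when the player character touches it.
; A BoxHit overlap by a BP_char, gated on a valid owner other than that character, adds WG_InteractKing to the viewport for five seconds.
; An IsActive flag blocks repeat triggers until the widget is removed.
; BeginPlay caches the player's BP_char, though the graph never reads it.
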(event OnComponentBeginOverlap(BoxHit)
  (params (OverlappedComponent :type Primitive%20Component%20Object%20Reference) (OtherActor :type Actor%20Object%20Reference) (OtherComp :type Primitive%20Component%20Object%20Reference) (OtherBodyIndex :type Integer) (bFromSweep :type Boolean) (SweepResult :type Hit%20Result%20Structure%20%28by%20ref%29))
  (bind _returnvalue (Components|GetOwner))
  (Utilities|IsValid _returnvalue
    (:Is%20Valid
      (if (not (== _returnvalue OtherActor))
        (Utilities|Casting|CastToBP_char OtherActor)
        (if (not (Variables|Default|GetIsActive))
          (bind _returnvalue_2 (UserInterface|CreateWidget "/Game/Blueprints/HUD/WG_InteractKing.WG_InteractKing_C" (Game|GetPlayerController 0)))
          (Variables|Default|SetIsActive true)
          (bind _output_get (Variables|Default|SetDialogMenu _returnvalue_2))
          (UserInterface|Viewport|AddtoViewport _output_get 0)
          (Utilities|FlowControl|Delay 5.0)
          (Widget|RemovefromParent _output_get)
          (Variables|Default|SetIsActive false))))))

(event EventBeginPlay
  (bind _asbp_char (Utilities|Casting|CastToBP_char (Game|GetPlayerCharacter 0)))
  (Variables|Default|SetChar _asbp_char))

(event Collision|EventActorBeginOverlap
  (params (OtherActor :type Actor%20Object%20Reference)))

(event EventTick
  (params (DeltaSeconds :type Float%20%28single-precision%29)))

(fn ConstructionScript)