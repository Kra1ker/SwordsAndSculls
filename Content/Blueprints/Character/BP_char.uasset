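; Player character for a 2D side-scroller, with double jump, held dash, and light and heavy ground attacks.
; Input moves it along X, velocity sets left/right facing, and actions jump directly to animation nodes.
; Attacks and landings stop and lock movement, with delays gating repeat attacks.
; Damage updates health through a dispatcher call and knocks it away from EnemyPos, while death triggers a delayed respawn at the starting location.
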(event Custom|Respawn
  (Class|PaperZDAnimInstance|JumptoNode (Variables|/Script/PaperZD.PaperZDAnimationComponent|GetAnimInstance (Variables|Default|GetAnimationComponent)) "None" "None")
  (Transformation|SetActorLocation (Variables|Default|GetResp_Location) false false)
  (Variables|Default|SetIsDeath false)
  (Components|Activation|SetActive (Variables|Character|GetCharacterMovement) true false)
  (Variables|Default|SetHealth 1e+02)
  (Default|CallChangingHealth (/ (Variables|Default|GetHealth) (Variables|Default|GetMax_Health))))

(event EventBeginPlay
  (Variables|Default|SetResp_Location (Transformation|GetActorLocation))
  (bind _asplayer_controller (Utilities|Casting|CastToPlayerController (Pawn|GetController)))
  (bind _returnvalue (UserInterface|CreateWidget "/Game/Blueprints/HUD/WG_Hud.WG_Hud_C" _asplayer_controller))
  (UserInterface|Viewport|AddtoViewport _returnvalue 0))

(event Collision|EventActorBeginOverlap
  (params (OtherActor :type Actor%20Object%20Reference)))

(event Game|Damage|EventAnyDamage
  (params (Damage :type Float%20%28single-precision%29) (DamageType :type Damage%20Type%20Object%20Reference) (InstigatedBy :type Controller%20Object%20Reference) (DamageCauser :type Actor%20Object%20Reference))
  (if (not (Variables|Default|GetIsDeath))
    (bind _output_get (Variables|Default|SetHealth (- (Variables|Default|GetHealth) Damage)))
    (Development|PrintString (Utilities|String|Append "Health: " (Utilities|String|ToString(Integer) (Math|Float|Truncate _output_get))))
    (Default|CallChangingHealth (/ (Variables|Default|GetHealth) (Variables|Default|GetMax_Health)))
    (if (> (Variables|Default|GetHealth) 0)
      (Math|Float|CompareFloat (.x (Transformation|GetWorldLocation (Variables|Default|GetSprite))) (Variables|Default|GetEnemyPos)
        (:>
          (Character|LaunchCharacter "500.000000,0.000000,250.000000" true false))
        (:<
          (Character|LaunchCharacter "-500.000000,0.000000,250.000000" true false)))
      (else
        (Variables|Default|SetIsDeath true)
        (Components|Activation|SetActive (Variables|Character|GetCharacterMovement) false false)
        (Class|PaperZDAnimInstance|JumptoNode (Variables|/Script/PaperZD.PaperZDAnimationComponent|GetAnimInstance (Variables|Default|GetAnimationComponent)) "Death" "None")
        (Utilities|FlowControl|Delay 0.8)
        (CallFunction|Respawn)))))

(event EventOnJumped
  ;[1 1 1] Jumping Animation
  (Class|PaperZDAnimInstance|JumptoNode (Variables|/Script/PaperZD.PaperZDAnimationComponent|GetAnimInstance (Variables|Default|GetAnimationComponent)) "Jump" "None"))

(event EventOnWalkingOffLedge
  (params (PreviousFloorImpactNormal :type Vector%20%28by%20ref%29 :default "0, 0, 0") (PreviousFloorContactNormal :type Vector%20%28by%20ref%29 :default "0, 0, 0") (PreviousLocation :type Vector%20%28by%20ref%29 :default "0, 0, 0") (TimeDelta :type Float%20%28single-precision%29))
  ;[1 1 1] Jumping Animation
  (Class|PaperZDAnimInstance|JumptoNode (Variables|/Script/PaperZD.PaperZDAnimationComponent|GetAnimInstance (Variables|Default|GetAnimationComponent)) "Jump" "None"))

(event EventOnLanded
  (params (Hit :type Hit%20Result%20Structure%20%28by%20ref%29))
  ;[1 1 1] Landing
  (Class|PaperZDAnimInstance|JumptoNode (Variables|/Script/PaperZD.PaperZDAnimationComponent|GetAnimInstance (Variables|Default|GetAnimationComponent)) "Landed" "None")
  (Components|Movement|StopMovementImmediately (Variables|Character|GetCharacterMovement))
  (Variables|Default|SetIsMovementLock true))

(event EventTick
  (params (DeltaSeconds :type Float%20%28single-precision%29))
  (bind _returnvalue (Pawn|GetController))
  (bind _returnvalue_2 (Pawn|GetController))
  ;[1 1 1] Rotation
  (if (not (Variables|Default|GetIsMovementLock))
    (Math|Float|CompareFloat (.x (Variables|/Script/Engine.MovementComponent|GetVelocity (Variables|Character|GetCharacterMovement))) 0.0
      (:>
        ;;[1 1 1] Right
        (Utilities|IsValid _returnvalue_2
          (:Is%20Valid
            (Pawn|SetControlRotation _returnvalue_2 (Math|Rotator|MakeRotator 0.0 0.0 0.0)))))
      (:<
        ;;[1 1 1] Left
        (Utilities|IsValid _returnvalue
          (:Is%20Valid
            (Pawn|SetControlRotation _returnvalue (Math|Rotator|MakeRotator 0.0 0.0 1.8e+02))))))))

(event Input|ActionEvents|InputActionDash
  (params (Key :type Key%20Structure :default "None"))
  ;[1 1 1] Dash
  (:Pressed
    (Variables|Default|SetRunPlayerRate 1.5)
    (Variables|/Script/Engine.CharacterMovementComponent|SetMaxWalkSpeed (Variables|Character|GetCharacterMovement) 1e+03))
  (:Released
    (Variables|Default|SetRunPlayerRate 1.0)
    (Variables|/Script/Engine.CharacterMovementComponent|SetMaxWalkSpeed (Variables|Character|GetCharacterMovement) 6.5e+02)))

(event Input|ActionEvents|InputActionJump
  (params (Key :type Key%20Structure :default "None"))
  ;[1 1 1] Jumping Action
  (:Pressed
    (Variables|Default|SetJumpMaxCount 2)
    (Variables|Default|SetJumpMaxHoldTime 0.0)
    (Character|Jump))
  (:Released
    (Character|StopJumping)))

(event Input|ActionEvents|InputActionHeavyattack
  (params (Key :type Key%20Structure :default "None"))
  (:Pressed
    (if (and (not (Variables|Default|GetIsAttacking)) (AI|Components|NavMovement|IsMovingonGround (Variables|Character|GetCharacterMovement)))
      (Variables|Default|SetIsAttacking true)
      (Class|PaperZDAnimInstance|JumptoNode (Variables|/Script/PaperZD.PaperZDAnimationComponent|GetAnimInstance (Variables|Default|GetAnimationComponent)) "H_Attack" "None")
      (Components|Movement|StopMovementImmediately (Variables|Character|GetCharacterMovement))
      (Variables|Default|SetIsMovementLock true)
      (Utilities|FlowControl|Delay 0.9)
      (Variables|Default|SetIsAttacking false))))

(event Input|ActionEvents|InputActionLightattack
  (params (Key :type Key%20Structure :default "None"))
  (:Pressed
    (if (and (not (Variables|Default|GetIsAttacking)) (AI|Components|NavMovement|IsMovingonGround (Variables|Character|GetCharacterMovement)))
      (Variables|Default|SetIsAttacking true)
      (Class|PaperZDAnimInstance|JumptoNode (Variables|/Script/PaperZD.PaperZDAnimationComponent|GetAnimInstance (Variables|Default|GetAnimationComponent)) "L_Attack" "None")
      (Components|Movement|StopMovementImmediately (Variables|Character|GetCharacterMovement))
      (Variables|Default|SetIsMovementLock true)
      (Utilities|FlowControl|Delay 0.5)
      (Variables|Default|SetIsAttacking false))))

(event Input|AxisEvents|InputAxisRight/left
  (params (AxisValue :type Float%20%28single-precision%29))
  ;[1 1 1] Movement
  (if (not (Variables|Default|GetIsMovementLock))
    (Pawn|Input|AddMovementInput "0.800000,0.000000,0.000000" AxisValue false)))

(fn ConstructionScript)